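; BP_Present is the gift actor that animates its drop in front of a house and triggers the level completion sequence.
; On spawn, the FloatAndScale timeline drives the mesh's scale, float height and movement, while Tick spins it by a fixed per-frame step.
; When the timeline finishes, it calls ReverseMech on BP_MainGamePawn and shows an animated completion widget: Level 3's own, or Level 1's for any other level.
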(event EventBeginPlay
  ;[1 1 1] Beginplay of Smooth Spawning and Dropping In front of House
  (bind (_direction _scale _floating _housemovement) (Timeline|FloatAndScale PlayFromStart)
    (:Update
      (Transformation|SetRelativeScale3D (Variables|Default|GetPresent) (Math|Conversions|ToVector(Float) _scale))
      (Transformation|SetRelativeLocation (Variables|Default|GetPresent) (Math|Vector|MakeVector _housemovement 0.0 _floating) false false))
    (:Finished
      (bind _asbp_main_game_pawn (Utilities|Casting|CastToBP_MainGamePawn (Game|Player|GetPlayerPawn 0)))
      (Default|ReverseMech _asbp_main_game_pawn)
      (bind _output_get (Variables|Default|SetLevel%20Number (Variables|/Game/Blueprints/Character/BP_MainGamePawn.BP_MainGamePawn_C|GetLevelNumber _asbp_main_game_pawn)))
      (if (== _output_get 3)
        (bind _returnvalue (UserInterface|CreateWidget "/Game/Blueprints/Widget/LevelsEndWidget/WBP_Level3Completed.WBP_Level3Completed_C"))
        (UserInterface|Viewport|AddtoViewport _returnvalue 0)
        (UserInterface|Animation|PlayAnimation _returnvalue (Variables|/Game/Blueprints/Widget/LevelsEndWidget/WBP_Level3Completed.WBP_Level3Completed_C|GetMC_Anim _returnvalue) 0.0 1 "Forward" 1.0 false)
        (else
          (bind _returnvalue_2 (UserInterface|CreateWidget "/Game/Blueprints/Widget/LevelsEndWidget/WBP_Level1Completed.WBP_Level1Completed_C"))
          (UserInterface|Viewport|AddtoViewport _returnvalue_2 0)
          (UserInterface|Animation|PlayAnimation _returnvalue_2 (Variables|/Game/Blueprints/Widget/LevelsEndWidget/WBP_Level1Completed.WBP_Level1Completed_C|GetMC_Anim _returnvalue_2) 0.0 1 "Forward" 1.0 false))))))

(event EventTick
  (params (DeltaSeconds :type Float%20%28single-precision%29))
  ;[1 1 1] Tick Event For Rotation
  (Transformation|AddLocalRotation (Variables|Default|GetPresent) "0.000000,1.500000,0.000000" false false))

(fn ConstructionScript)