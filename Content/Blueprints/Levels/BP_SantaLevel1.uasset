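; Santa level 1 actor that runs timed platform movement, two-way teleports and the level ending.
; Thirteen seconds after BeginPlay, staggered timelines lerp seven components far downward.
; Two start/end box pairs teleport BP_Santa to arrows, swapping Pawn collision so only one side triggers, while RotationControl disables controller yaw.
; The final Box calls BP_MainPawn's CloseUp, then Santa's End; Tick copies four pawn axis flags into branches that do nothing.
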(event OnComponentBeginOverlap(FirstStartBox)
  (params (OverlappedComponent :type Primitive%20Component%20Object%20Reference) (OtherActor :type Actor%20Object%20Reference) (OtherComp :type Primitive%20Component%20Object%20Reference) (OtherBodyIndex :type Integer) (bFromSweep :type Boolean) (SweepResult :type Hit%20Result%20Structure%20%28by%20ref%29))
  (bind _asbp_santa (Utilities|Casting|CastToBP_Santa OtherActor))
  (Variables|/Script/Engine.Pawn|SetbUseControllerRotationYaw _asbp_santa false)
  (Transformation|SetActorLocation _asbp_santa (Transformation|GetWorldLocation (Variables|Default|GetFirstStartArrow)) false false)
  (Utilities|FlowControl|Delay 1.0)
  (Variables|/Script/Engine.Pawn|SetbUseControllerRotationYaw _asbp_santa true)
  (Collision|SetCollisionResponsetoChannel (Variables|Default|GetFirstEndBox) "ECC_Pawn" "ECR_Overlap")
  (Collision|SetCollisionResponsetoChannel (Variables|Default|GetFirstStartBox) "ECC_Pawn" "ECR_Ignore"))

(event OnComponentBeginOverlap(FirstEndBox)
  (params (OverlappedComponent :type Primitive%20Component%20Object%20Reference) (OtherActor :type Actor%20Object%20Reference) (OtherComp :type Primitive%20Component%20Object%20Reference) (OtherBodyIndex :type Integer) (bFromSweep :type Boolean) (SweepResult :type Hit%20Result%20Structure%20%28by%20ref%29))
  (bind _asbp_santa (Utilities|Casting|CastToBP_Santa OtherActor))
  (Variables|/Script/Engine.Pawn|SetbUseControllerRotationYaw _asbp_santa false)
  (Transformation|SetActorLocation _asbp_santa (Transformation|GetWorldLocation (Variables|Default|GetFirstEndArrow)) false false)
  (Utilities|FlowControl|Delay 1.0)
  (Variables|/Script/Engine.Pawn|SetbUseControllerRotationYaw _asbp_santa true)
  (Collision|SetCollisionResponsetoChannel (Variables|Default|GetFirstEndBox) "ECC_Pawn" "ECR_Ignore")
  (Collision|SetCollisionResponsetoChannel (Variables|Default|GetFirstStartBox) "ECC_Pawn" "ECR_Overlap"))

(event OnComponentBeginOverlap(RotationControl)
  (params (OverlappedComponent :type Primitive%20Component%20Object%20Reference) (OtherActor :type Actor%20Object%20Reference) (OtherComp :type Primitive%20Component%20Object%20Reference) (OtherBodyIndex :type Integer) (bFromSweep :type Boolean) (SweepResult :type Hit%20Result%20Structure%20%28by%20ref%29))
  (bind _asbp_santa (Utilities|Casting|CastToBP_Santa OtherActor))
  (Variables|/Script/Engine.Pawn|SetbUseControllerRotationYaw _asbp_santa false))

(event OnComponentBeginOverlap(SecondStartBox)
  (params (OverlappedComponent :type Primitive%20Component%20Object%20Reference) (OtherActor :type Actor%20Object%20Reference) (OtherComp :type Primitive%20Component%20Object%20Reference) (OtherBodyIndex :type Integer) (bFromSweep :type Boolean) (SweepResult :type Hit%20Result%20Structure%20%28by%20ref%29))
  (bind _asbp_santa (Utilities|Casting|CastToBP_Santa OtherActor))
  (Variables|/Script/Engine.Pawn|SetbUseControllerRotationYaw _asbp_santa false)
  (Transformation|SetActorLocation _asbp_santa (Transformation|GetWorldLocation (Variables|Default|GetSecondStartArrow)) false false)
  (Utilities|FlowControl|Delay 1.0)
  (Variables|/Script/Engine.Pawn|SetbUseControllerRotationYaw _asbp_santa true)
  (Collision|SetCollisionResponsetoChannel (Variables|Default|GetSecondEndBox) "ECC_Pawn" "ECR_Overlap")
  (Collision|SetCollisionResponsetoChannel (Variables|Default|GetSecondStartBox) "ECC_Pawn" "ECR_Ignore"))

(event OnComponentBeginOverlap(SecondEndBox)
  (params (OverlappedComponent :type Primitive%20Component%20Object%20Reference) (OtherActor :type Actor%20Object%20Reference) (OtherComp :type Primitive%20Component%20Object%20Reference) (OtherBodyIndex :type Integer) (bFromSweep :type Boolean) (SweepResult :type Hit%20Result%20Structure%20%28by%20ref%29))
  (bind _asbp_santa (Utilities|Casting|CastToBP_Santa OtherActor))
  (Variables|/Script/Engine.Pawn|SetbUseControllerRotationYaw _asbp_santa false)
  (Transformation|SetActorLocation _asbp_santa (Transformation|GetWorldLocation (Variables|Default|GetSecondEndArrow)) false false)
  (Utilities|FlowControl|Delay 1.0)
  (Variables|/Script/Engine.Pawn|SetbUseControllerRotationYaw _asbp_santa true)
  (Collision|SetCollisionResponsetoChannel (Variables|Default|GetSecondEndBox) "ECC_Pawn" "ECR_Ignore")
  (Collision|SetCollisionResponsetoChannel (Variables|Default|GetSecondStartBox) "ECC_Pawn" "ECR_Overlap"))

(event OnComponentBeginOverlap(Box)
  (params (OverlappedComponent :type Primitive%20Component%20Object%20Reference) (OtherActor :type Actor%20Object%20Reference) (OtherComp :type Primitive%20Component%20Object%20Reference) (OtherBodyIndex :type Integer) (bFromSweep :type Boolean) (SweepResult :type Hit%20Result%20Structure%20%28by%20ref%29))
  (bind _asbp_santa (Utilities|Casting|CastToBP_Santa OtherActor))
  (bind _asbp_main_pawn (Utilities|Casting|CastToBP_MainPawn (Game|Player|GetPlayerPawn 0)))
  (Default|CloseUp _asbp_main_pawn)
  (Utilities|FlowControl|Delay 5.0)
  (Default|End _asbp_santa))

(event Custom|AxisThree
  (params (Axis3 :type Boolean))
  (Variables|Default|SetAxis3 Axis3)
  (if (Variables|Default|GetAxis3)
    _))

(event Custom|AxisZero
  (params (Axis0 :type Boolean))
  (Variables|Default|SetAxis0 Axis0)
  (if (Variables|Default|GetAxis0)
    _))

(event Custom|AxisOne
  (params (Axis1 :type Boolean))
  (Variables|Default|SetAxis1 Axis1)
  (if (Variables|Default|GetAxis1)
    _))

(event Custom|AxisTwo
  (params (Axis2 :type Boolean))
  (Variables|Default|SetAxis2 Axis2)
  (if (Variables|Default|GetAxis2)
    _))

(event EventBeginPlay
  (Input|EnableInput (Game|GetPlayerController 0) 0)
  (Collision|SetCollisionResponsetoChannel (Variables|Default|GetFirstEndBox) "ECC_Pawn" "ECR_Ignore")
  (Collision|SetCollisionResponsetoChannel (Variables|Default|GetSecondEndBox) "ECC_Pawn" "ECR_Ignore")
  (Utilities|FlowControl|Delay 13.0)
  (Utilities|FlowControl|Sequence
    (:then_0
      (bind _shiftpos (Timeline|PlatformDis PlayFromStart)
        (:Update
          (Transformation|SetRelativeLocation (Variables|Default|Get1) (Math|Vector|Lerp(Vector) (Variables|/Script/Engine.SceneComponent|GetRelativeLocation (Variables|Default|Get1)) "1180.000000,600.000000,-10000.000000" _shiftpos) false false))))
    (:then_1
      (Utilities|FlowControl|Delay 0.1)
      (bind _shiftpos_2 (Timeline|Timeline PlayFromStart)
        (:Update
          (Transformation|SetRelativeLocation (Variables|Default|Get2) (Math|Vector|Lerp(Vector) (Variables|/Script/Engine.SceneComponent|GetRelativeLocation (Variables|Default|Get2)) "1370.000000,600.000000,-10000.000000" _shiftpos_2) false false))))
    (:then_2
      (Utilities|FlowControl|Delay 0.2)
      (bind _shiftpos_3 (Timeline|Timeline_0 PlayFromStart)
        (:Update
          (Transformation|SetRelativeLocation (Variables|Default|Get3) (Math|Vector|Lerp(Vector) (Variables|/Script/Engine.SceneComponent|GetRelativeLocation (Variables|Default|Get3)) "1560.000000,600.000000,-10000.000000" _shiftpos_3) false false))))
    (:then_3
      (Utilities|FlowControl|Delay 0.3)
      (bind _shiftpos_4 (Timeline|Timeline_1 PlayFromStart)
        (:Update
          (Transformation|SetRelativeLocation (Variables|Default|Get4) (Math|Vector|Lerp(Vector) (Variables|/Script/Engine.SceneComponent|GetRelativeLocation (Variables|Default|Get4)) "1750.000000,600.000000,-10000.000000" _shiftpos_4) false false))))
    (:then_4
      (Utilities|FlowControl|Delay 0.4)
      (bind _shiftpos_5 (Timeline|Timeline_2 PlayFromStart)
        (:Update
          (Transformation|SetRelativeLocation (Variables|Default|Get5) (Math|Vector|Lerp(Vector) (Variables|/Script/Engine.SceneComponent|GetRelativeLocation (Variables|Default|Get5)) "1940.000000,600.000000,-10000.000000" _shiftpos_5) false false))))
    (:then_5
      (Utilities|FlowControl|Delay 0.5)
      (bind _shiftpos_6 (Timeline|Timeline_3 PlayFromStart)
        (:Update
          (Transformation|SetRelativeLocation (Variables|Default|Get6) (Math|Vector|Lerp(Vector) (Variables|/Script/Engine.SceneComponent|GetRelativeLocation (Variables|Default|Get6)) "2130.000000,600.000000,-10000.000000" _shiftpos_6) false false))))
    (:then_6
      (Utilities|FlowControl|Delay 0.6)
      (bind _shiftpos_7 (Timeline|Timeline_4 PlayFromStart)
        (:Update
          (Transformation|SetRelativeLocation (Variables|Default|Get7) (Math|Vector|Lerp(Vector) (Variables|/Script/Engine.SceneComponent|GetRelativeLocation (Variables|Default|Get7)) "2320.000000,600.000000,-10000.000000" _shiftpos_7) false false))))))

(event EventTick
  (params (DeltaSeconds :type Float%20%28single-precision%29))
  (bind _asbp_main_pawn (Utilities|Casting|CastToBP_MainPawn (Game|Player|GetPlayerPawn 0)))
  (Variables|Default|SetAxis0 (Variables|/Game/Blueprints/Character/BP_MainPawn.BP_MainPawn_C|GetAxisZero _asbp_main_pawn))
  (Variables|Default|SetAxis1 (Variables|/Game/Blueprints/Character/BP_MainPawn.BP_MainPawn_C|GetAxisOne _asbp_main_pawn))
  (Variables|Default|SetAxis2 (Variables|/Game/Blueprints/Character/BP_MainPawn.BP_MainPawn_C|GetAxisTwo _asbp_main_pawn))
  (Variables|Default|SetAxis3 (Variables|/Game/Blueprints/Character/BP_MainPawn.BP_MainPawn_C|GetAxisThree _asbp_main_pawn))
  (if (Variables|Default|GetAxis0)
    _
    (else
      _))
  (CallFunction|AxisZero (Variables|Default|GetAxis0))
  (if (Variables|Default|GetAxis1)
    _
    (else
      _))
  (CallFunction|AxisOne (Variables|Default|GetAxis1))
  (if (Variables|Default|GetAxis2)
    _
    (else
      _))
  (CallFunction|AxisTwo (Variables|Default|GetAxis2))
  (if (Variables|Default|GetAxis3)
    _
    (else
      _))
  (CallFunction|AxisThree (Variables|Default|GetAxis3)))

(fn ConstructionScript)