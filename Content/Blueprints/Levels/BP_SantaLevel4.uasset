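; Level 4 puzzle Blueprint that routes BP_Santa to a present delivery, whose overlap triggers the pawn's close-up, then Santa's End.
; Two start/end box pairs teleport Santa to arrows, alternately toggling Pawn collision to control travel direction.
; Per-camera-axis events stop Santa and move four blocking cubes in or out of play.
; Cube hits feed DoOnce input-mode changes, which holding left mouse resets through Tick.
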(event OnComponentBeginOverlap(FirstStartBox)
  (params (OverlappedComponent :type Primitive%20Component%20Object%20Reference) (OtherActor :type Actor%20Object%20Reference) (OtherComp :type Primitive%20Component%20Object%20Reference) (OtherBodyIndex :type Integer) (bFromSweep :type Boolean) (SweepResult :type Hit%20Result%20Structure%20%28by%20ref%29))
  ;[1 1 1] Overlap Events of Start And End Box
  (bind _asbp_santa (Utilities|Casting|CastToBP_Santa OtherActor))
  (Transformation|SetActorLocation _asbp_santa (Transformation|GetWorldLocation (Variables|Default|GetFirstStartArrow)) false false)
  (Utilities|FlowControl|Delay 0.25)
  (Collision|SetCollisionResponsetoChannel (Variables|Default|GetFirstEndBox) "ECC_Pawn" "ECR_Overlap")
  (Collision|SetCollisionResponsetoChannel (Variables|Default|GetFirstStartBox) "ECC_Pawn" "ECR_Ignore"))

(event OnComponentBeginOverlap(FirstEndBox)
  (params (OverlappedComponent :type Primitive%20Component%20Object%20Reference) (OtherActor :type Actor%20Object%20Reference) (OtherComp :type Primitive%20Component%20Object%20Reference) (OtherBodyIndex :type Integer) (bFromSweep :type Boolean) (SweepResult :type Hit%20Result%20Structure%20%28by%20ref%29))
  ;[1 1 1] Overlap Events of Start And End Box
  (bind _asbp_santa (Utilities|Casting|CastToBP_Santa OtherActor))
  (Transformation|SetActorLocation _asbp_santa (Transformation|GetWorldLocation (Variables|Default|GetFirstEndArrow)) false false)
  (Utilities|FlowControl|Delay 0.25)
  (Collision|SetCollisionResponsetoChannel (Variables|Default|GetFirstEndBox) "ECC_Pawn" "ECR_Ignore")
  (Collision|SetCollisionResponsetoChannel (Variables|Default|GetFirstStartBox) "ECC_Pawn" "ECR_Overlap"))

(event OnComponentHit(BlockingCubeOne)
  (params (HitComponent :type Primitive%20Component%20Object%20Reference) (OtherActor :type Actor%20Object%20Reference) (OtherComp :type Primitive%20Component%20Object%20Reference) (NormalImpulse :type Vector :default "0, 0, 0") (Hit :type Hit%20Result%20Structure%20%28by%20ref%29))
  ;[1 1 1] Hit Events For Blocking Cubes
  (Utilities|Casting|CastToBP_Santa OtherActor)
  (Utilities|FlowControl|DoOnce false
    (:Completed
      (Input|SetInputModeGameandUI (Game|GetPlayerController 0) 0 "DoNotLock" false false))))

(event OnComponentBeginOverlap(SecondStartBox)
  (params (OverlappedComponent :type Primitive%20Component%20Object%20Reference) (OtherActor :type Actor%20Object%20Reference) (OtherComp :type Primitive%20Component%20Object%20Reference) (OtherBodyIndex :type Integer) (bFromSweep :type Boolean) (SweepResult :type Hit%20Result%20Structure%20%28by%20ref%29))
  ;[1 1 1] Overlap Events of Start And End Box
  (bind _asbp_santa (Utilities|Casting|CastToBP_Santa OtherActor))
  (Transformation|SetActorLocation _asbp_santa (Transformation|GetWorldLocation (Variables|Default|GetSecondStartArrow)) false false)
  (Utilities|FlowControl|Delay 0.25)
  (Collision|SetCollisionResponsetoChannel (Variables|Default|GetSecondEndBox) "ECC_Pawn" "ECR_Overlap")
  (Collision|SetCollisionResponsetoChannel (Variables|Default|GetSecondStartBox) "ECC_Pawn" "ECR_Ignore"))

(event OnComponentBeginOverlap(SecondEndBox)
  (params (OverlappedComponent :type Primitive%20Component%20Object%20Reference) (OtherActor :type Actor%20Object%20Reference) (OtherComp :type Primitive%20Component%20Object%20Reference) (OtherBodyIndex :type Integer) (bFromSweep :type Boolean) (SweepResult :type Hit%20Result%20Structure%20%28by%20ref%29))
  ;[1 1 1] Overlap Events of Start And End Box
  (bind _asbp_santa (Utilities|Casting|CastToBP_Santa OtherActor))
  (Transformation|SetActorLocation _asbp_santa (Transformation|GetWorldLocation (Variables|Default|GetSecondEndArrow)) false false)
  (Utilities|FlowControl|Delay 0.25)
  (Collision|SetCollisionResponsetoChannel (Variables|Default|GetSecondEndBox) "ECC_Pawn" "ECR_Ignore")
  (Collision|SetCollisionResponsetoChannel (Variables|Default|GetSecondStartBox) "ECC_Pawn" "ECR_Overlap"))

(event OnComponentBeginOverlap(DeliveringPresent)
  (params (OverlappedComponent :type Primitive%20Component%20Object%20Reference) (OtherActor :type Actor%20Object%20Reference) (OtherComp :type Primitive%20Component%20Object%20Reference) (OtherBodyIndex :type Integer) (bFromSweep :type Boolean) (SweepResult :type Hit%20Result%20Structure%20%28by%20ref%29))
  ;[1 1 1] Overlap Event Of Present
  (bind _asbp_santa (Utilities|Casting|CastToBP_Santa OtherActor))
  (bind _asbp_main_game_pawn (Utilities|Casting|CastToBP_MainGamePawn (Game|Player|GetPlayerPawn 0)))
  (Default|CloseUp _asbp_main_game_pawn)
  (Utilities|FlowControl|Delay 5.0)
  (Default|End _asbp_santa))

(event OnComponentHit(BlockingCubeTwo)
  (params (HitComponent :type Primitive%20Component%20Object%20Reference) (OtherActor :type Actor%20Object%20Reference) (OtherComp :type Primitive%20Component%20Object%20Reference) (NormalImpulse :type Vector :default "0, 0, 0") (Hit :type Hit%20Result%20Structure%20%28by%20ref%29))
  ;[1 1 1] Hit Events For Blocking Cubes
  (Utilities|Casting|CastToBP_Santa OtherActor)
  (Utilities|FlowControl|DoOnce false
    (:Completed
      (Input|SetInputModeGameandUI (Game|GetPlayerController 0) 0 "DoNotLock" false false))))

(event OnComponentHit(BlockingCubeThree)
  (params (HitComponent :type Primitive%20Component%20Object%20Reference) (OtherActor :type Actor%20Object%20Reference) (OtherComp :type Primitive%20Component%20Object%20Reference) (NormalImpulse :type Vector :default "0, 0, 0") (Hit :type Hit%20Result%20Structure%20%28by%20ref%29))
  ;[1 1 1] Hit Events For Blocking Cubes
  (Utilities|Casting|CastToBP_Santa OtherActor)
  (Utilities|FlowControl|DoOnce false
    (:Completed
      (Input|SetInputModeGameandUI (Game|GetPlayerController 0) 0 "DoNotLock" false false))))

(event OnComponentHit(BlockingCubeFour)
  (params (HitComponent :type Primitive%20Component%20Object%20Reference) (OtherActor :type Actor%20Object%20Reference) (OtherComp :type Primitive%20Component%20Object%20Reference) (NormalImpulse :type Vector :default "0, 0, 0") (Hit :type Hit%20Result%20Structure%20%28by%20ref%29))
  ;[1 1 1] Hit Events For Blocking Cubes
  (Utilities|Casting|CastToBP_Santa OtherActor)
  (Utilities|FlowControl|DoOnce false
    (:Completed
      (Input|SetInputModeGameandUI (Game|GetPlayerController 0) 0 "DoNotLock" false false))))

(event Custom|AxisThree
  (bind _blockingcubethree (Variables|Default|GetBlockingCubeThree))
  (bind _blockingcubeone (Variables|Default|GetBlockingCubeOne))
  ;[1 1 1] Events For Every Cam Axis
  (Class|NavMovementComponent|StopActiveMovement (Variables|/Script/Engine.Character|GetCharacterMovement (Variables|Default|GetSantaRef)))
  (Collision|SetCollisionResponsetoAllChannels _blockingcubeone "ECR_Block")
  (Transformation|SetRelativeLocation _blockingcubeone "450.000000,990.000000,195.000000" false false)
  (Transformation|SetRelativeLocation (Variables|Default|GetBlockingCubeTwo) "361.000000,1010.000000,315.000000" false false)
  (Collision|SetCollisionResponsetoAllChannels _blockingcubethree "ECR_Block")
  (Transformation|SetRelativeLocation _blockingcubethree "-130.000000,980.000000,125.000000" false false)
  (Transformation|SetRelativeLocation (Variables|Default|GetBlockingCubeFour) "-40.000000,1010.000000,265.000000" false false))

(event Custom|AxisZero
  (bind _blockingcubeone (Variables|Default|GetBlockingCubeOne))
  (bind _blockingcubethree (Variables|Default|GetBlockingCubeThree))
  ;[1 1 1] Events For Every Cam Axis
  (Class|NavMovementComponent|StopActiveMovement (Variables|/Script/Engine.Character|GetCharacterMovement (Variables|Default|GetSantaRef)))
  (Collision|SetCollisionResponsetoAllChannels _blockingcubeone "ECR_Ignore")
  (Transformation|SetRelativeLocation _blockingcubeone "450.000000,990.000000,10000.000000" false false)
  (Transformation|SetRelativeLocation (Variables|Default|GetBlockingCubeTwo) "361.000000,1010.000000,10000.000000" false false)
  (Collision|SetCollisionResponsetoAllChannels _blockingcubethree "ECR_Block")
  (Transformation|SetRelativeLocation _blockingcubethree "-130.000000,980.000000,125.000000" false false)
  (Transformation|SetRelativeLocation (Variables|Default|GetBlockingCubeFour) "-40.000000,1010.000000,265.000000" false false))

(event Custom|AxisOne
  (bind _blockingcubeone (Variables|Default|GetBlockingCubeOne))
  (bind _blockingcubethree (Variables|Default|GetBlockingCubeThree))
  ;[1 1 1] Events For Every Cam Axis
  (Class|NavMovementComponent|StopActiveMovement (Variables|/Script/Engine.Character|GetCharacterMovement (Variables|Default|GetSantaRef)))
  (Collision|SetCollisionResponsetoAllChannels _blockingcubeone "ECR_Block")
  (Transformation|SetRelativeLocation _blockingcubeone "450.000000,990.000000,195.000000" false false)
  (Transformation|SetRelativeLocation (Variables|Default|GetBlockingCubeTwo) "361.000000,1010.000000,315.000000" false false)
  (Collision|SetCollisionResponsetoAllChannels _blockingcubethree "ECR_Ignore")
  (Transformation|SetRelativeLocation _blockingcubethree "-130.000000,980.000000,10000.000000" false false)
  (Transformation|SetRelativeLocation (Variables|Default|GetBlockingCubeFour) "-40.000000,1010.000000,10000.000000" false false))

(event Custom|UnlockingInput
  ;[1 1 1] Hit Events For Blocking Cubes
  (Utilities|FlowControl|Sequence
    (:then_0
      (Utilities|FlowControl|DoOnce false) ; enters at Reset
    )
    (:then_1
      (Utilities|FlowControl|DoOnce false) ; enters at Reset
    )
    (:then_2
      (Utilities|FlowControl|DoOnce false) ; enters at Reset
    )
    (:then_3
      (Utilities|FlowControl|DoOnce false) ; enters at Reset
    )
    (:then_4)))

(event Custom|AxisTwo
  (bind _blockingcubeone (Variables|Default|GetBlockingCubeOne))
  (bind _blockingcubethree (Variables|Default|GetBlockingCubeThree))
  ;[1 1 1] Events For Every Cam Axis
  (Class|NavMovementComponent|StopActiveMovement (Variables|/Script/Engine.Character|GetCharacterMovement (Variables|Default|GetSantaRef)))
  (Collision|SetCollisionResponsetoAllChannels _blockingcubeone "ECR_Block")
  (Transformation|SetRelativeLocation _blockingcubeone "450.000000,990.000000,195.000000" false false)
  (Transformation|SetRelativeLocation (Variables|Default|GetBlockingCubeTwo) "361.000000,1010.000000,315.000000" false false)
  (Collision|SetCollisionResponsetoAllChannels _blockingcubethree "ECR_Block")
  (Transformation|SetRelativeLocation _blockingcubethree "-130.000000,980.000000,125.000000" false false)
  (Transformation|SetRelativeLocation (Variables|Default|GetBlockingCubeFour) "-40.000000,1010.000000,265.000000" false false))

(event EventBeginPlay
  ;[1 1 1] Beginplay & Tick
  (Input|EnableInput (Game|GetPlayerController 0) 0)
  (Collision|SetCollisionResponsetoChannel (Variables|Default|GetFirstEndBox) "ECC_Pawn" "ECR_Ignore")
  (Collision|SetCollisionResponsetoChannel (Variables|Default|GetSecondEndBox) "ECC_Pawn" "ECR_Ignore")
  (Utilities|FlowControl|Delay 13.0))

(event EventTick
  (params (DeltaSeconds :type Float%20%28single-precision%29))
  ;[1 1 1] Beginplay & Tick
  (bind _asbp_main_game_pawn (Utilities|Casting|CastToBP_MainGamePawn (Game|Player|GetPlayerPawn 0)))
  (Variables|Default|SetAxis0 (Variables|/Game/Blueprints/Character/BP_MainGamePawn.BP_MainGamePawn_C|GetAxisZero _asbp_main_game_pawn))
  (Variables|Default|SetAxis1 (Variables|/Game/Blueprints/Character/BP_MainGamePawn.BP_MainGamePawn_C|GetAxisOne _asbp_main_game_pawn))
  (Variables|Default|SetAxis2 (Variables|/Game/Blueprints/Character/BP_MainGamePawn.BP_MainGamePawn_C|GetAxisTwo _asbp_main_game_pawn))
  (Variables|Default|SetAxis3 (Variables|/Game/Blueprints/Character/BP_MainGamePawn.BP_MainGamePawn_C|GetAxisThree _asbp_main_game_pawn))
  (if (Game|Player|IsInputKeyDown (Game|GetPlayerController 0) "LeftMouseButton")
    (CallFunction|UnlockingInput)))

(fn ConstructionScript)