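; Main menu pawn that drives the camera and UI for a five-stage level-select screen.
; Events start, return from or step between stages, using timelines to move the camera and adjust ortho width while MenuPlatformRef plays matching sequences.
; Each transition creates and animates stage, play, options or quit widgets, usually switching to UI-only input.
; BeginPlay loads the BP_SantaJourney save so stages two and three can show locked or unlocked animations.
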(event Custom|StartLevel
  (bind _camera (Variables|Default|GetCamera))
  (bind _camera_2 (Variables|Default|GetCamera))
  (bind _camera_3 (Variables|Default|GetCamera))
  (bind _camera_4 (Variables|Default|GetCamera))
  (bind _camera_5 (Variables|Default|GetCamera))
  ;[1 1 1] ProcessBetweenStartLevelButton
  (switch int (Variables|Default|GetStandingLevelRef)
    (:1
      (if (== (Variables|/Game/Blueprints/Levels/BP_MainMenu.BP_MainMenu_C|GetStandingLevel (Variables|Default|GetMenuPlatformRef)) 1)
        (Utilities|FlowControl|Sequence
          (:then_0
            (bind (_direction _camerapos _camerawidth) (Timeline|Level1SelectionCamera PlayFromStart)
              (:Update
                (Transformation|SetRelativeLocation _camera_2 _camerapos false false)
                (Class|CameraComponent|SetOrthoWidth _camera_2 _camerawidth))))
          (:then_1
            (Class|ActorSequenceComponent|PlaySequence (Variables|/Game/Blueprints/Levels/BP_MainMenu.BP_MainMenu_C|GetLevel1Beg (Variables|Default|GetMenuPlatformRef)))
            (bind _returnvalue (UserInterface|CreateWidget "/Game/Blueprints/Widget/LevelsWidget/WBP_Level1.WBP_Level1_C"))
            (bind _output_get (Variables|Default|SetStage1WidgetRef _returnvalue))
            (UserInterface|Viewport|AddtoViewport _output_get 0)
            (UserInterface|Animation|PlayAnimation (Variables|Default|GetStage1WidgetRef) (Variables|/Game/Blueprints/Widget/LevelsWidget/WBP_Level1.WBP_Level1_C|GetStageOneAnim (Variables|Default|GetStage1WidgetRef)) 0.0 1 "Forward" 1.0 false)
            (Utilities|FlowControl|Delay 2.0)
            (Input|SetInputModeUIOnly (Game|GetPlayerController 0) 0 "DoNotLock" false)))))
    (:2
      (if (== (Variables|/Game/Blueprints/Levels/BP_MainMenu.BP_MainMenu_C|GetStandingLevel (Variables|Default|GetMenuPlatformRef)) 2)
        (Utilities|FlowControl|Sequence
          (:then_0
            (bind (_direction_2 _camerapos_2 _camerawidth_2) (Timeline|Level2SelectionCamera PlayFromStart)
              (:Update
                (Transformation|SetRelativeLocation _camera_3 _camerapos_2 false false)
                (Class|CameraComponent|SetOrthoWidth _camera_3 _camerawidth_2))))
          (:then_1
            (Class|ActorSequenceComponent|PlaySequence (Variables|/Game/Blueprints/Levels/BP_MainMenu.BP_MainMenu_C|GetLevel2Beg (Variables|Default|GetMenuPlatformRef)))
            (bind _returnvalue_2 (UserInterface|CreateWidget "/Game/Blueprints/Widget/LevelsWidget/WBP_Level2.WBP_Level2_C"))
            (bind _output_get_2 (Variables|Default|SetStage2WidgetRef _returnvalue_2))
            (UserInterface|Viewport|AddtoViewport _output_get_2 0)
            (if (not (Variables|Default|GetLevel%202Unlocked))
              (UserInterface|Animation|PlayAnimation (Variables|Default|GetStage2WidgetRef) (Variables|/Game/Blueprints/Widget/LevelsWidget/WBP_Level2.WBP_Level2_C|GetStageTwoLockedAnim (Variables|Default|GetStage2WidgetRef)) 0.0 1 "Forward" 1.0 false)
              (Utilities|FlowControl|Delay 2.0)
              (Input|SetInputModeUIOnly (Game|GetPlayerController 0) 0 "DoNotLock" false)
              (else
                (UserInterface|Animation|PlayAnimation (Variables|Default|GetStage2WidgetRef) (Variables|/Game/Blueprints/Widget/LevelsWidget/WBP_Level2.WBP_Level2_C|GetStageTwoAnim (Variables|Default|GetStage2WidgetRef)) 0.0 1 "Forward" 1.0 false)
                (Utilities|FlowControl|Delay 2.0)
                (Input|SetInputModeUIOnly (Game|GetPlayerController 0) 0 "DoNotLock" false)))))))
    (:3
      (if (== (Variables|/Game/Blueprints/Levels/BP_MainMenu.BP_MainMenu_C|GetStandingLevel (Variables|Default|GetMenuPlatformRef)) 3)
        (Utilities|FlowControl|Sequence
          (:then_0
            (bind (_direction_3 _camerapos_3 _camerawidth_3) (Timeline|Level3SelectionCamera PlayFromStart)
              (:Update
                (Transformation|SetRelativeLocation _camera_4 _camerapos_3 false false)
                (Class|CameraComponent|SetOrthoWidth _camera_4 _camerawidth_3))))
          (:then_1
            (Class|ActorSequenceComponent|PlaySequence (Variables|/Game/Blueprints/Levels/BP_MainMenu.BP_MainMenu_C|GetLevel3Beg (Variables|Default|GetMenuPlatformRef)))
            (bind _returnvalue_3 (UserInterface|CreateWidget "/Game/Blueprints/Widget/LevelsWidget/WBP_Level3.WBP_Level3_C"))
            (bind _output_get_3 (Variables|Default|SetStage3WidgetRef _returnvalue_3))
            (UserInterface|Viewport|AddtoViewport _output_get_3 0)
            (if (not (Variables|Default|GetLevel%203Unlocked))
              (UserInterface|Animation|PlayAnimation (Variables|Default|GetStage3WidgetRef) (Variables|/Game/Blueprints/Widget/LevelsWidget/WBP_Level3.WBP_Level3_C|GetStageThreeLockedAnim (Variables|Default|GetStage3WidgetRef)) 0.0 1 "Forward" 1.0 false)
              (Utilities|FlowControl|Delay 2.0)
              (Input|SetInputModeUIOnly (Game|GetPlayerController 0) 0 "DoNotLock" false)
              (else
                (UserInterface|Animation|PlayAnimation (Variables|Default|GetStage3WidgetRef) (Variables|/Game/Blueprints/Widget/LevelsWidget/WBP_Level3.WBP_Level3_C|GetStageThreeAnim (Variables|Default|GetStage3WidgetRef)) 0.0 1 "Forward" 1.0 false)
                (Utilities|FlowControl|Delay 2.0)
                (Input|SetInputModeUIOnly (Game|GetPlayerController 0) 0 "DoNotLock" false)))))))
    (:4
      (if (== (Variables|/Game/Blueprints/Levels/BP_MainMenu.BP_MainMenu_C|GetStandingLevel (Variables|Default|GetMenuPlatformRef)) 4)
        (Utilities|FlowControl|Sequence
          (:then_0
            (bind (_direction_4 _camerapos_4 _camerawidth_4) (Timeline|Level4SelectionCamera PlayFromStart)
              (:Update
                (Transformation|SetRelativeLocation _camera_5 _camerapos_4 false false)
                (Class|CameraComponent|SetOrthoWidth _camera_5 _camerawidth_4))))
          (:then_1
            (Class|ActorSequenceComponent|PlaySequence (Variables|/Game/Blueprints/Levels/BP_MainMenu.BP_MainMenu_C|GetLevel4Beg (Variables|Default|GetMenuPlatformRef)))
            (bind _returnvalue_4 (UserInterface|CreateWidget "/Game/Blueprints/Widget/LevelsWidget/WBP_Level4.WBP_Level4_C"))
            (bind _output_get_4 (Variables|Default|SetStage4WidgetRef _returnvalue_4))
            (UserInterface|Viewport|AddtoViewport _output_get_4 0)
            (UserInterface|Animation|PlayAnimation (Variables|Default|GetStage4WidgetRef) (Variables|/Game/Blueprints/Widget/LevelsWidget/WBP_Level4.WBP_Level4_C|GetStageFourAnim (Variables|Default|GetStage4WidgetRef)) 0.0 1 "Forward" 1.0 false)
            (Utilities|FlowControl|Delay 2.0)
            (Input|SetInputModeUIOnly (Game|GetPlayerController 0) 0 "DoNotLock" false)))))
    (:5
      (if (== (Variables|/Game/Blueprints/Levels/BP_MainMenu.BP_MainMenu_C|GetStandingLevel (Variables|Default|GetMenuPlatformRef)) 5)
        (Utilities|FlowControl|Sequence
          (:then_0
            (bind (_direction_5 _camerapos_5 _camerawidth_5) (Timeline|Level5SelectionCamera PlayFromStart)
              (:Update
                (Transformation|SetRelativeLocation _camera _camerapos_5 false false)
                (Class|CameraComponent|SetOrthoWidth _camera _camerawidth_5))))
          (:then_1
            (Class|ActorSequenceComponent|PlaySequence (Variables|/Game/Blueprints/Levels/BP_MainMenu.BP_MainMenu_C|GetLevel5Beg (Variables|Default|GetMenuPlatformRef)))
            (bind _returnvalue_5 (UserInterface|CreateWidget "/Game/Blueprints/Widget/LevelsWidget/WBP_Level5.WBP_Level5_C"))
            (bind _output_get_5 (Variables|Default|SetStage5WidgetRef _returnvalue_5))
            (UserInterface|Viewport|AddtoViewport _output_get_5 0)
            (UserInterface|Animation|PlayAnimation (Variables|Default|GetStage5WidgetRef) (Variables|/Game/Blueprints/Widget/LevelsWidget/WBP_Level5.WBP_Level5_C|GetStageFiveAnim (Variables|Default|GetStage5WidgetRef)) 0.0 1 "Forward" 1.0 false)
            (Utilities|FlowControl|Delay 2.0)
            (Input|SetInputModeUIOnly (Game|GetPlayerController 0) 0 "DoNotLock" false)))))))

(event Custom|OptionsMenu
  ;[1 1 1] Options Menu
  (bind _returnvalue (UserInterface|CreateWidget "/Game/Blueprints/Widget/WBP_Options.WBP_Options_C"))
  (bind _output_get (Variables|Default|SetOptionsWidgetRef _returnvalue))
  (UserInterface|Viewport|AddtoViewport _output_get 0)
  (UserInterface|Animation|PlayAnimation (Variables|Default|GetOptionsWidgetRef) (Variables|/Game/Blueprints/Widget/WBP_Options.WBP_Options_C|GetCommonAnim (Variables|Default|GetOptionsWidgetRef)) 0.0 1 "Forward" 1.0 false)
  (Input|SetInputModeUIOnly (Game|GetPlayerController 0) 0 "DoNotLock" false))

(event Custom|Reverse4-3
  ;[1 1 1] NextLevelCamAndWidgetMec
  (bind _camerapos (Timeline|Level3-4 ReverseFromEnd)
    (:Update
      (Transformation|SetRelativeLocation (Variables|Default|GetCamera) _camerapos false false))))

(event Custom|Reverse5-4
  ;[1 1 1] NextLevelCamAndWidgetMec
  (bind _camerapos (Timeline|Level4-5 ReverseFromEnd)
    (:Update
      (Transformation|SetRelativeLocation (Variables|Default|GetCamera) _camerapos false false))))

(event Custom|Level1Return
  (bind _camera (Variables|Default|GetCamera))
  ;[1 1 1] ProcessBetweenStartLevelButton
  (bind (_direction _camerapos _camerawidth) (Timeline|Level1SelectionCamera ReverseFromEnd)
    (:Update
      (Transformation|SetRelativeLocation _camera _camerapos false false)
      (Class|CameraComponent|SetOrthoWidth _camera _camerawidth))))

(event Custom|Level2Return
  (bind _camera (Variables|Default|GetCamera))
  ;[1 1 1] ProcessBetweenStartLevelButton
  (bind (_direction _camerapos _camerawidth) (Timeline|Level2SelectionCamera ReverseFromEnd)
    (:Update
      (Transformation|SetRelativeLocation _camera _camerapos false false)
      (Class|CameraComponent|SetOrthoWidth _camera _camerawidth))))

(event Custom|Level3Return
  (bind _camera (Variables|Default|GetCamera))
  ;[1 1 1] ProcessBetweenStartLevelButton
  (bind (_direction _camerapos _camerawidth) (Timeline|Level3SelectionCamera ReverseFromEnd)
    (:Update
      (Transformation|SetRelativeLocation _camera _camerapos false false)
      (Class|CameraComponent|SetOrthoWidth _camera _camerawidth))))

(event Custom|Level4Return
  (bind _camera (Variables|Default|GetCamera))
  ;[1 1 1] ProcessBetweenStartLevelButton
  (bind (_direction _camerapos _camerawidth) (Timeline|Level4SelectionCamera ReverseFromEnd)
    (:Update
      (Transformation|SetRelativeLocation _camera _camerapos false false)
      (Class|CameraComponent|SetOrthoWidth _camera _camerawidth))))

(event Custom|Level5Return
  (bind _camera (Variables|Default|GetCamera))
  ;[1 1 1] ProcessBetweenStartLevelButton
  (bind (_direction _camerapos _camerawidth) (Timeline|Level5SelectionCamera ReverseFromEnd)
    (:Update
      (Transformation|SetRelativeLocation _camera _camerapos false false)
      (Class|CameraComponent|SetOrthoWidth _camera _camerawidth))))

(event Custom|OpenLevel
  ;[1 1 1] Open Level
  (switch int (Variables|Default|GetStandingLevelRef)
    (:1
      (Default|PathtoLevel1 (Variables|Default|GetMenuPlatformRef)))
    (:2
      (Default|PathtoLevel2 (Variables|Default|GetMenuPlatformRef)))
    (:3
      (Default|PathtoLevel3 (Variables|Default|GetMenuPlatformRef)))
    (:4
      (Default|PathtoLevel4 (Variables|Default|GetMenuPlatformRef)))
    (:5
      (Default|PathtoLevel5 (Variables|Default|GetMenuPlatformRef)))))

(event Custom|QuitMenu
  ;[1 1 1] Quiting Menu And Return From Quit Menu
  (bind _returnvalue (UserInterface|CreateWidget "/Game/Blueprints/Widget/WBP_Quit.WBP_Quit_C"))
  (bind _output_get (Variables|Default|SetQuitWidgetRef _returnvalue))
  (UserInterface|Viewport|AddtoViewport _output_get 0)
  (UserInterface|Animation|PlayAnimation (Variables|Default|GetQuitWidgetRef) (Variables|/Game/Blueprints/Widget/WBP_Quit.WBP_Quit_C|GetExitInvokeAnim (Variables|Default|GetQuitWidgetRef)) 0.0 1 "Forward" 1.0 false)
  (Utilities|FlowControl|Delay 1.5)
  (Input|SetInputModeUIOnly (Game|GetPlayerController 0) 0 "DoNotLock" false))

(event Custom|ReturnFromQuit
  ;[1 1 1] Quiting Menu And Return From Quit Menu
  (bind _returnvalue (UserInterface|CreateWidget "/Game/Blueprints/Widget/WBP_Play.WBP_Play_C"))
  (bind _output_get (Variables|Default|SetPlayWidgetRef _returnvalue))
  (UserInterface|Viewport|AddtoViewport _output_get 0)
  (UserInterface|Animation|PlayAnimation (Variables|Default|GetPlayWidgetRef) (Variables|/Game/Blueprints/Widget/WBP_Play.WBP_Play_C|GetBeginningAnim (Variables|Default|GetPlayWidgetRef)) 0.0 1 "Forward" 1.0 false)
  (Utilities|FlowControl|Delay 1.5)
  (Input|SetInputModeUIOnly (Game|GetPlayerController 0) 0 "DoNotLock" false))

(event Custom|ReturnFromOptions
  ;[1 1 1] Options Menu
  (bind _returnvalue (UserInterface|CreateWidget "/Game/Blueprints/Widget/WBP_Play.WBP_Play_C"))
  (bind _output_get (Variables|Default|SetPlayWidgetRef _returnvalue))
  (UserInterface|Viewport|AddtoViewport _output_get 0)
  (UserInterface|Animation|PlayAnimation (Variables|Default|GetPlayWidgetRef) (Variables|/Game/Blueprints/Widget/WBP_Play.WBP_Play_C|GetBeginningAnim (Variables|Default|GetPlayWidgetRef)) 0.0 1 "Forward" 1.0 false)
  (Utilities|FlowControl|Delay 1.5)
  (Input|SetInputModeUIOnly (Game|GetPlayerController 0) 0 "DoNotLock" false))

(event Custom|ReturnFromLevel
  ;[1 1 1] ProcessBetweenReturnToMainMenuButton
  (Utilities|FlowControl|Sequence
    (:then_0
      (switch int (Variables|Default|GetStandingLevelRef)
        (:1
          (CallFunction|Level1Return)
          (Class|ActorSequenceComponent|PlaySequence (Variables|/Game/Blueprints/Levels/BP_MainMenu.BP_MainMenu_C|GetLevel1End (Variables|Default|GetMenuPlatformRef))))
        (:2
          (CallFunction|Level2Return)
          (Class|ActorSequenceComponent|PlaySequence (Variables|/Game/Blueprints/Levels/BP_MainMenu.BP_MainMenu_C|GetLevel2End (Variables|Default|GetMenuPlatformRef))))
        (:3
          (CallFunction|Level3Return)
          (Class|ActorSequenceComponent|PlaySequence (Variables|/Game/Blueprints/Levels/BP_MainMenu.BP_MainMenu_C|GetLevel3End (Variables|Default|GetMenuPlatformRef))))
        (:4
          (CallFunction|Level4Return)
          (Class|ActorSequenceComponent|PlaySequence (Variables|/Game/Blueprints/Levels/BP_MainMenu.BP_MainMenu_C|GetLevel4End (Variables|Default|GetMenuPlatformRef))))
        (:5
          (CallFunction|Level5Return)
          (Class|ActorSequenceComponent|PlaySequence (Variables|/Game/Blueprints/Levels/BP_MainMenu.BP_MainMenu_C|GetLevel5End (Variables|Default|GetMenuPlatformRef))))))
    (:then_1
      (bind _returnvalue (UserInterface|CreateWidget "/Game/Blueprints/Widget/WBP_Play.WBP_Play_C"))
      (bind _output_get (Variables|Default|SetPlayWidgetRef _returnvalue))
      (UserInterface|Viewport|AddtoViewport _output_get 0)
      (UserInterface|Animation|PlayAnimation (Variables|Default|GetPlayWidgetRef) (Variables|/Game/Blueprints/Widget/WBP_Play.WBP_Play_C|GetBeginningAnim (Variables|Default|GetPlayWidgetRef)) 0.0 1 "Forward" 1.0 false)
      (Utilities|FlowControl|Delay 1.5)
      (Input|SetInputModeUIOnly (Game|GetPlayerController 0) 0 "DoNotLock" false))))

(event Custom|NextLevel
  ;[1 1 1] NextLevelCamAndWidgetMec
  (switch int (Variables|Default|GetStandingLevelRef)
    (:1
      (Default|OnetoTwo (Variables|Default|GetMenuPlatformRef))
      (Utilities|FlowControl|Sequence
        (:then_0
          (bind _camerapos (Timeline|Level1-2 PlayFromStart)
            (:Update
              (Transformation|SetRelativeLocation (Variables|Default|GetCamera) _camerapos false false))))
        (:then_1
          (Class|ActorSequenceComponent|PlaySequence (Variables|/Game/Blueprints/Levels/BP_MainMenu.BP_MainMenu_C|GetLevel1-2Path (Variables|Default|GetMenuPlatformRef)))
          (Utilities|FlowControl|Delay 3.5)
          (bind _returnvalue (UserInterface|CreateWidget "/Game/Blueprints/Widget/LevelsWidget/WBP_Level2.WBP_Level2_C"))
          (bind _output_get (Variables|Default|SetStage2WidgetRef _returnvalue))
          (UserInterface|Viewport|AddtoViewport _output_get 0)
          (if (not (Variables|Default|GetLevel%202Unlocked))
            (UserInterface|Animation|PlayAnimation (Variables|Default|GetStage2WidgetRef) (Variables|/Game/Blueprints/Widget/LevelsWidget/WBP_Level2.WBP_Level2_C|GetStageTwoLockedAnim (Variables|Default|GetStage2WidgetRef)) 0.0 1 "Forward" 1.0 false)
            (else
              (UserInterface|Animation|PlayAnimation (Variables|Default|GetStage2WidgetRef) (Variables|/Game/Blueprints/Widget/LevelsWidget/WBP_Level2.WBP_Level2_C|GetStageTwoAnim (Variables|Default|GetStage2WidgetRef)) 0.0 1 "Forward" 1.0 false))))))
    (:2
      (Default|TwotoThree (Variables|Default|GetMenuPlatformRef))
      (Utilities|FlowControl|Sequence
        (:then_0
          (bind _camerapos_2 (Timeline|Level2-3 PlayFromStart)
            (:Update
              (Transformation|SetRelativeLocation (Variables|Default|GetCamera) _camerapos_2 false false))))
        (:then_1
          (Class|ActorSequenceComponent|PlaySequence (Variables|/Game/Blueprints/Levels/BP_MainMenu.BP_MainMenu_C|GetLevel2-3Path (Variables|Default|GetMenuPlatformRef)))
          (Utilities|FlowControl|Delay 3.5)
          (bind _returnvalue_2 (UserInterface|CreateWidget "/Game/Blueprints/Widget/LevelsWidget/WBP_Level3.WBP_Level3_C"))
          (bind _output_get_2 (Variables|Default|SetStage3WidgetRef _returnvalue_2))
          (UserInterface|Viewport|AddtoViewport _output_get_2 0)
          (if (not (Variables|Default|GetLevel%203Unlocked))
            (UserInterface|Animation|PlayAnimation (Variables|Default|GetStage3WidgetRef) (Variables|/Game/Blueprints/Widget/LevelsWidget/WBP_Level3.WBP_Level3_C|GetStageThreeLockedAnim (Variables|Default|GetStage3WidgetRef)) 0.0 1 "Forward" 1.0 false)
            (else
              (UserInterface|Animation|PlayAnimation (Variables|Default|GetStage3WidgetRef) (Variables|/Game/Blueprints/Widget/LevelsWidget/WBP_Level3.WBP_Level3_C|GetStageThreeAnim (Variables|Default|GetStage3WidgetRef)) 0.0 1 "Forward" 1.0 false))))))
    (:3
      (Default|ThreetoFour (Variables|Default|GetMenuPlatformRef))
      (Utilities|FlowControl|Sequence
        (:then_0
          (bind _camerapos_3 (Timeline|Level3-4 PlayFromStart)
            (:Update
              (Transformation|SetRelativeLocation (Variables|Default|GetCamera) _camerapos_3 false false))))
        (:then_1
          (Class|ActorSequenceComponent|PlaySequence (Variables|/Game/Blueprints/Levels/BP_MainMenu.BP_MainMenu_C|GetLevel3-4Path (Variables|Default|GetMenuPlatformRef)))
          (Utilities|FlowControl|Delay 3.5)
          (bind _returnvalue_3 (UserInterface|CreateWidget "/Game/Blueprints/Widget/LevelsWidget/WBP_Level4.WBP_Level4_C"))
          (bind _output_get_3 (Variables|Default|SetStage4WidgetRef _returnvalue_3))
          (UserInterface|Viewport|AddtoViewport _output_get_3 0)
          (UserInterface|Animation|PlayAnimation (Variables|Default|GetStage4WidgetRef) (Variables|/Game/Blueprints/Widget/LevelsWidget/WBP_Level4.WBP_Level4_C|GetStageFourAnim (Variables|Default|GetStage4WidgetRef)) 0.0 1 "Forward" 1.0 false))))
    (:4
      (Default|FourtoFive (Variables|Default|GetMenuPlatformRef))
      (Utilities|FlowControl|Sequence
        (:then_0
          (bind _camerapos_4 (Timeline|Level4-5 PlayFromStart)
            (:Update
              (Transformation|SetRelativeLocation (Variables|Default|GetCamera) _camerapos_4 false false))))
        (:then_1
          (Class|ActorSequenceComponent|PlaySequence (Variables|/Game/Blueprints/Levels/BP_MainMenu.BP_MainMenu_C|GetLevel4-5Path (Variables|Default|GetMenuPlatformRef)))
          (Utilities|FlowControl|Delay 3.5)
          (bind _returnvalue_4 (UserInterface|CreateWidget "/Game/Blueprints/Widget/LevelsWidget/WBP_Level5.WBP_Level5_C"))
          (bind _output_get_4 (Variables|Default|SetStage5WidgetRef _returnvalue_4))
          (UserInterface|Viewport|AddtoViewport _output_get_4 0)
          (UserInterface|Animation|PlayAnimation (Variables|Default|GetStage5WidgetRef) (Variables|/Game/Blueprints/Widget/LevelsWidget/WBP_Level5.WBP_Level5_C|GetStageFiveAnim (Variables|Default|GetStage5WidgetRef)) 0.0 1 "Forward" 1.0 false))))))

(event Custom|PreLevel
  ;[1 1 1] PreviousLevelCamAndWidgetMec
  (switch int (Variables|Default|GetStandingLevelRef)
    (:2
      (Default|TwotoOne (Variables|Default|GetMenuPlatformRef))
      (Utilities|FlowControl|Sequence
        (:then_0
          (CallFunction|Reverse2-1)
          (Class|ActorSequenceComponent|PlaySequence (Variables|/Game/Blueprints/Levels/BP_MainMenu.BP_MainMenu_C|GetLevel2-1Path (Variables|Default|GetMenuPlatformRef))))
        (:then_1
          (Utilities|FlowControl|Delay 3.5)
          (bind _returnvalue (UserInterface|CreateWidget "/Game/Blueprints/Widget/LevelsWidget/WBP_Level1.WBP_Level1_C"))
          (bind _output_get (Variables|Default|SetStage1WidgetRef _returnvalue))
          (UserInterface|Viewport|AddtoViewport _output_get 0)
          (UserInterface|Animation|PlayAnimation (Variables|Default|GetStage1WidgetRef) (Variables|/Game/Blueprints/Widget/LevelsWidget/WBP_Level1.WBP_Level1_C|GetStageOneAnim (Variables|Default|GetStage1WidgetRef)) 0.0 1 "Forward" 1.0 false))))
    (:3
      (Default|ThreetoTwo (Variables|Default|GetMenuPlatformRef))
      (Utilities|FlowControl|Sequence
        (:then_0
          (CallFunction|Reverse3-2)
          (Class|ActorSequenceComponent|PlaySequence (Variables|/Game/Blueprints/Levels/BP_MainMenu.BP_MainMenu_C|GetLevel3-2Path (Variables|Default|GetMenuPlatformRef))))
        (:then_1
          (Utilities|FlowControl|Delay 3.5)
          (bind _returnvalue_2 (UserInterface|CreateWidget "/Game/Blueprints/Widget/LevelsWidget/WBP_Level2.WBP_Level2_C"))
          (bind _output_get_2 (Variables|Default|SetStage2WidgetRef _returnvalue_2))
          (UserInterface|Viewport|AddtoViewport _output_get_2 0)
          (if (not (Variables|Default|GetLevel%202Unlocked))
            (UserInterface|Animation|PlayAnimation (Variables|Default|GetStage2WidgetRef) (Variables|/Game/Blueprints/Widget/LevelsWidget/WBP_Level2.WBP_Level2_C|GetStageTwoLockedAnim (Variables|Default|GetStage2WidgetRef)) 0.0 1 "Forward" 1.0 false)
            (else
              (UserInterface|Animation|PlayAnimation (Variables|Default|GetStage2WidgetRef) (Variables|/Game/Blueprints/Widget/LevelsWidget/WBP_Level2.WBP_Level2_C|GetStageTwoAnim (Variables|Default|GetStage2WidgetRef)) 0.0 1 "Forward" 1.0 false))))))
    (:4
      (Default|FourtoThree (Variables|Default|GetMenuPlatformRef))
      (Utilities|FlowControl|Sequence
        (:then_0
          (CallFunction|Reverse4-3)
          (Class|ActorSequenceComponent|PlaySequence (Variables|/Game/Blueprints/Levels/BP_MainMenu.BP_MainMenu_C|GetLevel4-3Path (Variables|Default|GetMenuPlatformRef))))
        (:then_1
          (Utilities|FlowControl|Delay 3.5)
          (bind _returnvalue_3 (UserInterface|CreateWidget "/Game/Blueprints/Widget/LevelsWidget/WBP_Level3.WBP_Level3_C"))
          (bind _output_get_3 (Variables|Default|SetStage3WidgetRef _returnvalue_3))
          (UserInterface|Viewport|AddtoViewport _output_get_3 0)
          (if (not (Variables|Default|GetLevel%203Unlocked))
            (UserInterface|Animation|PlayAnimation (Variables|Default|GetStage3WidgetRef) (Variables|/Game/Blueprints/Widget/LevelsWidget/WBP_Level3.WBP_Level3_C|GetStageThreeLockedAnim (Variables|Default|GetStage3WidgetRef)) 0.0 1 "Forward" 1.0 false)
            (else
              (UserInterface|Animation|PlayAnimation (Variables|Default|GetStage3WidgetRef) (Variables|/Game/Blueprints/Widget/LevelsWidget/WBP_Level3.WBP_Level3_C|GetStageThreeAnim (Variables|Default|GetStage3WidgetRef)) 0.0 1 "Forward" 1.0 false))))))
    (:5
      (Default|FivetoFour (Variables|Default|GetMenuPlatformRef))
      (Utilities|FlowControl|Sequence
        (:then_0
          (CallFunction|Reverse5-4)
          (Class|ActorSequenceComponent|PlaySequence (Variables|/Game/Blueprints/Levels/BP_MainMenu.BP_MainMenu_C|GetLevel5-4Path (Variables|Default|GetMenuPlatformRef))))
        (:then_1
          (Utilities|FlowControl|Delay 3.5)
          (bind _returnvalue_4 (UserInterface|CreateWidget "/Game/Blueprints/Widget/LevelsWidget/WBP_Level4.WBP_Level4_C"))
          (bind _output_get_4 (Variables|Default|SetStage4WidgetRef _returnvalue_4))
          (UserInterface|Viewport|AddtoViewport _output_get_4 0)
          (UserInterface|Animation|PlayAnimation (Variables|Default|GetStage4WidgetRef) (Variables|/Game/Blueprints/Widget/LevelsWidget/WBP_Level4.WBP_Level4_C|GetStageFourAnim (Variables|Default|GetStage4WidgetRef)) 0.0 1 "Forward" 1.0 false))))))

(event Custom|Reverse2-1
  ;[1 1 1] NextLevelCamAndWidgetMec
  (bind _camerapos (Timeline|Level1-2 ReverseFromEnd)
    (:Update
      (Transformation|SetRelativeLocation (Variables|Default|GetCamera) _camerapos false false))))

(event Custom|Reverse3-2
  ;[1 1 1] NextLevelCamAndWidgetMec
  (bind _camerapos (Timeline|Level2-3 ReverseFromEnd)
    (:Update
      (Transformation|SetRelativeLocation (Variables|Default|GetCamera) _camerapos false false))))

(event EventBeginPlay
  ;[1 1 1] BeginPlay
  (Transformation|SetRelativeLocation (Variables|Default|GetCamera) "315.000000,0.000000,390.000000" false false)
  (bind _returnvalue (SaveGame|LoadGamefromSlot "Levels"))
  (bind _asbp_santa_journey (Utilities|Casting|CastToBP_SantaJourney _returnvalue))
  (Variables|Default|SetLevel%202Unlocked (Variables|/Game/Blueprints/Saves/BP_SantaJourney.BP_SantaJourney_C|GetLevel2Unlocked _asbp_santa_journey))
  (Variables|Default|SetLevel%203Unlocked (Variables|/Game/Blueprints/Saves/BP_SantaJourney.BP_SantaJourney_C|GetLevel3Unlocked _asbp_santa_journey)))

(fn ConstructionScript)