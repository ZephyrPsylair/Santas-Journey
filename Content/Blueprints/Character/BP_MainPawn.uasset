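; Main pawn with an orthographic camera that snaps smoothly between four isometric corner views on Left/Right input.
; A wrapping CameraPosition index selects a timeline that moves the boom offset and camera rotation, disabling input while it plays and updating Axis flags.
; BeginPlay runs a delayed zoom-out intro, then shows a WBP_Fade guide, whose Platform animation plays once on first A/D press.
; CloseUp and Reverse drive a reversible zoom timeline.
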(event Custom|CloseUp
  (bind (_direction _cam _camloc) (Timeline|CamMovement PlayFromStart)
    (:Update
      (Class|CameraComponent|SetOrthoWidth (Variables|Default|GetCamera) (Math|Float|Lerp 3e+03 1.5e+03 _cam))
      (Transformation|SetRelativeLocation (Variables|Default|GetCamera) (Math|Vector|Lerp(Vector) (Variables|/Script/Engine.SceneComponent|GetRelativeLocation (Variables|Default|GetCamera)) "-750.000000,-275.000000,0.000000" _camloc) false false))))

(event Custom|Reverse
  (bind (_direction _cam _camloc) (Timeline|CamMovement ReverseFromEnd)
    (:Update
      (Class|CameraComponent|SetOrthoWidth (Variables|Default|GetCamera) (Math|Float|Lerp 3e+03 1.5e+03 _cam))
      (Transformation|SetRelativeLocation (Variables|Default|GetCamera) (Math|Vector|Lerp(Vector) (Variables|/Script/Engine.SceneComponent|GetRelativeLocation (Variables|Default|GetCamera)) "-750.000000,-275.000000,0.000000" _camloc) false false))))

(event EventBeginPlay
  (bind _camera (Variables|Default|GetCamera))
  (Transformation|SetRelativeLocation (Variables|Default|GetCamera) "315.000000,0.000000,390.000000" false false)
  (Utilities|FlowControl|Delay 8.0)
  (Utilities|FlowControl|Sequence
    (:then_0
      (bind (_direction _camorthowidth _campos) (Timeline|SmoothPos Play)
        (:Update
          (Class|CameraComponent|SetOrthoWidth _camera (Math|Float|Lerp 1e+03 3e+03 _camorthowidth))
          (Transformation|SetRelativeLocation _camera (Math|Vector|Lerp(Vector) (Variables|/Script/Engine.SceneComponent|GetRelativeLocation (Variables|Default|GetCamera)) "0, 0, 0" _campos) false false))))
    (:then_1
      (Utilities|FlowControl|Delay 5.0)
      (bind _returnvalue (UserInterface|CreateWidget "/Game/Blueprints/Widget/WBP_Fade.WBP_Fade_C"))
      (bind _output_get (Variables|Default|SetGuideWidget _returnvalue))
      (UserInterface|Viewport|AddtoViewport _output_get 0)
      (UserInterface|Animation|PlayAnimation (Variables|Default|GetGuideWidget) (Variables|/Game/Blueprints/Widget/WBP_Fade.WBP_Fade_C|GetGuideAnim _returnvalue) 0.0 1 "Forward" 1.0 false))))

(event Collision|EventActorBeginOverlap
  (params (OtherActor :type Actor%20Object%20Reference)))

(event EventTick
  (params (DeltaSeconds :type Float%20%28single-precision%29))
  (bind _returnvalue (Game|GetPlayerController 0))
  (if (or (Game|Player|IsInputKeyDown _returnvalue "D") (Game|Player|IsInputKeyDown _returnvalue "A"))
    (Utilities|FlowControl|Sequence
      (:then_0
        (Utilities|FlowControl|DoOnce false
          (:Completed
            (UserInterface|Animation|PlayAnimation (Variables|Default|GetGuideWidget) (Variables|/Game/Blueprints/Widget/WBP_Fade.WBP_Fade_C|GetPlatform (Variables|Default|GetGuideWidget)) 0.0 1 "Forward" 1.0 false)))))))

(event Input|ActionEvents|InputActionRight
  (params (Key :type Key%20Structure :default "None"))
  (:Pressed
    (if (== (Variables|Default|GetCameraPosition) 3)
      (Variables|Default|SetCameraPosition 0)
      (else
        (Math|Integer|IncrementInt (Variables|Default|GetCameraPosition)
          (:%20%20
            _))))
    (switch int (Variables|Default|GetCameraPosition)
      (:0
        (Variables|Default|SetAxisThree false)
        (Variables|Default|SetAxisOne false)
        (bind _smoothrot (Timeline|SmoothRotation PlayFromStart)
          (:Update
            (Variables|/Script/Engine.SpringArmComponent|SetTargetOffset (Variables|Default|GetCameraBoom) (Math|Vector|Lerp(Vector) (Variables|/Script/Engine.SpringArmComponent|GetTargetOffset (Variables|Default|GetCameraBoom)) "0.000000,600.000000,600.000000" _smoothrot))
            (Transformation|SetRelativeRotation (Variables|Default|GetCamera) (Math|Interpolation|RInterpTo (Variables|/Script/Engine.SceneComponent|GetRelativeRotation (Variables|Default|GetCamera)) "-45.000000,-45.000000,0.000000" (Utilities|Time|GetWorldDeltaSeconds) 5.0) false false)
            (Input|DisableInput (Game|GetPlayerController 0)))
          (:Finished
            (Input|EnableInput (Game|GetPlayerController 0))
            (Variables|Default|SetAxisZero true))))
      (:1
        (Variables|Default|SetAxisTwo false)
        (Variables|Default|SetAxisZero false)
        (bind _smoothrot1 (Timeline|SmoothRotation1 PlayFromStart)
          (:Update
            (Variables|/Script/Engine.SpringArmComponent|SetTargetOffset (Variables|Default|GetCameraBoom) (Math|Vector|Lerp(Vector) (Variables|/Script/Engine.SpringArmComponent|GetTargetOffset (Variables|Default|GetCameraBoom)) "1200.000000,600.000000,600.000000" _smoothrot1))
            (Transformation|SetRelativeRotation (Variables|Default|GetCamera) (Math|Interpolation|RInterpTo (Variables|/Script/Engine.SceneComponent|GetRelativeRotation (Variables|Default|GetCamera)) "-45.000000,-135.000000,0.000000" (Utilities|Time|GetWorldDeltaSeconds) 5.0) false false)
            (Input|DisableInput (Game|GetPlayerController 0)))
          (:Finished
            (Input|EnableInput (Game|GetPlayerController 0))
            (Variables|Default|SetAxisOne true))))
      (:2
        (Variables|Default|SetAxisOne false)
        (Variables|Default|SetAxisThree false)
        (bind _smoothrot2 (Timeline|SmoothRotation2 PlayFromStart)
          (:Update
            (Variables|/Script/Engine.SpringArmComponent|SetTargetOffset (Variables|Default|GetCameraBoom) (Math|Vector|Lerp(Vector) (Variables|/Script/Engine.SpringArmComponent|GetTargetOffset (Variables|Default|GetCameraBoom)) "1200.000000,-600.000000,600.000000" _smoothrot2))
            (Transformation|SetRelativeRotation (Variables|Default|GetCamera) (Math|Interpolation|RInterpTo (Variables|/Script/Engine.SceneComponent|GetRelativeRotation (Variables|Default|GetCamera)) "-45.000000,135.000000,0.000000" (Utilities|Time|GetWorldDeltaSeconds) 5.0) false false)
            (Input|DisableInput (Game|GetPlayerController 0)))
          (:Finished
            (Input|EnableInput (Game|GetPlayerController 0))
            (Variables|Default|SetAxisTwo true))))
      (:3
        (Variables|Default|SetAxisTwo false)
        (Variables|Default|SetAxisZero false)
        (bind _smoothrot3 (Timeline|SmoothRotation3 PlayFromStart)
          (:Update
            (Variables|/Script/Engine.SpringArmComponent|SetTargetOffset (Variables|Default|GetCameraBoom) (Math|Vector|Lerp(Vector) (Variables|/Script/Engine.SpringArmComponent|GetTargetOffset (Variables|Default|GetCameraBoom)) "0.000000,-600.000000,600.000000" _smoothrot3))
            (Transformation|SetRelativeRotation (Variables|Default|GetCamera) (Math|Interpolation|RInterpTo (Variables|/Script/Engine.SceneComponent|GetRelativeRotation (Variables|Default|GetCamera)) "-45.000000,45.000000,0.000000" (Utilities|Time|GetWorldDeltaSeconds) 5.0) false false)
            (Input|DisableInput (Game|GetPlayerController 0)))
          (:Finished
            (Input|EnableInput (Game|GetPlayerController 0))
            (Variables|Default|SetAxisThree true)))))))

(event Input|ActionEvents|InputActionLeft
  (params (Key :type Key%20Structure :default "None"))
  (:Pressed
    (if (== (Variables|Default|GetCameraPosition) 0)
      (Variables|Default|SetCameraPosition 3)
      (else
        (Math|Integer|DecrementInt (Variables|Default|GetCameraPosition)
          (:%20%20
            _))))
    (switch int (Variables|Default|GetCameraPosition)
      (:0
        (Variables|Default|SetAxisThree false)
        (Variables|Default|SetAxisOne false)
        (bind _smoothrot (Timeline|SmoothRotation PlayFromStart)
          (:Update
            (Variables|/Script/Engine.SpringArmComponent|SetTargetOffset (Variables|Default|GetCameraBoom) (Math|Vector|Lerp(Vector) (Variables|/Script/Engine.SpringArmComponent|GetTargetOffset (Variables|Default|GetCameraBoom)) "0.000000,600.000000,600.000000" _smoothrot))
            (Transformation|SetRelativeRotation (Variables|Default|GetCamera) (Math|Interpolation|RInterpTo (Variables|/Script/Engine.SceneComponent|GetRelativeRotation (Variables|Default|GetCamera)) "-45.000000,-45.000000,0.000000" (Utilities|Time|GetWorldDeltaSeconds) 5.0) false false)
            (Input|DisableInput (Game|GetPlayerController 0)))
          (:Finished
            (Input|EnableInput (Game|GetPlayerController 0))
            (Variables|Default|SetAxisZero true))))
      (:1
        (Variables|Default|SetAxisTwo false)
        (Variables|Default|SetAxisZero false)
        (bind _smoothrot1 (Timeline|SmoothRotation1 PlayFromStart)
          (:Update
            (Variables|/Script/Engine.SpringArmComponent|SetTargetOffset (Variables|Default|GetCameraBoom) (Math|Vector|Lerp(Vector) (Variables|/Script/Engine.SpringArmComponent|GetTargetOffset (Variables|Default|GetCameraBoom)) "1200.000000,600.000000,600.000000" _smoothrot1))
            (Transformation|SetRelativeRotation (Variables|Default|GetCamera) (Math|Interpolation|RInterpTo (Variables|/Script/Engine.SceneComponent|GetRelativeRotation (Variables|Default|GetCamera)) "-45.000000,-135.000000,0.000000" (Utilities|Time|GetWorldDeltaSeconds) 5.0) false false)
            (Input|DisableInput (Game|GetPlayerController 0)))
          (:Finished
            (Input|EnableInput (Game|GetPlayerController 0))
            (Variables|Default|SetAxisOne true))))
      (:2
        (Variables|Default|SetAxisOne false)
        (Variables|Default|SetAxisThree false)
        (bind _smoothrot2 (Timeline|SmoothRotation2 PlayFromStart)
          (:Update
            (Variables|/Script/Engine.SpringArmComponent|SetTargetOffset (Variables|Default|GetCameraBoom) (Math|Vector|Lerp(Vector) (Variables|/Script/Engine.SpringArmComponent|GetTargetOffset (Variables|Default|GetCameraBoom)) "1200.000000,-600.000000,600.000000" _smoothrot2))
            (Transformation|SetRelativeRotation (Variables|Default|GetCamera) (Math|Interpolation|RInterpTo (Variables|/Script/Engine.SceneComponent|GetRelativeRotation (Variables|Default|GetCamera)) "-45.000000,135.000000,0.000000" (Utilities|Time|GetWorldDeltaSeconds) 5.0) false false)
            (Input|DisableInput (Game|GetPlayerController 0)))
          (:Finished
            (Input|EnableInput (Game|GetPlayerController 0))
            (Variables|Default|SetAxisTwo true))))
      (:3
        (Variables|Default|SetAxisTwo false)
        (Variables|Default|SetAxisZero false)
        (bind _smoothrot3 (Timeline|SmoothRotation3 PlayFromStart)
          (:Update
            (Variables|/Script/Engine.SpringArmComponent|SetTargetOffset (Variables|Default|GetCameraBoom) (Math|Vector|Lerp(Vector) (Variables|/Script/Engine.SpringArmComponent|GetTargetOffset (Variables|Default|GetCameraBoom)) "0.000000,-600.000000,600.000000" _smoothrot3))
            (Transformation|SetRelativeRotation (Variables|Default|GetCamera) (Math|Interpolation|RInterpTo (Variables|/Script/Engine.SceneComponent|GetRelativeRotation (Variables|Default|GetCamera)) "-45.000000,45.000000,0.000000" (Utilities|Time|GetWorldDeltaSeconds) 5.0) false false)
            (Input|DisableInput (Game|GetPlayerController 0)))
          (:Finished
            (Input|EnableInput (Game|GetPlayerController 0))
            (Variables|Default|SetAxisThree true)))))))

(fn ConstructionScript)