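; Turn-based toolkit action for game over, built to show DisplayText as center text on the player's HUD.
; PlayAction clears markers, then reaches a branch with a constant true condition that ends the action immediately.
; As a result, the HUD cast and DisplayCenterText call on the false side never run.
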(event EventPlayAction
  (CallFunction|ClearMarkers)
  (if true
    (CallFunction|EndAction true :!label _label)
    (else
      (bind _asbp_hud_atbtt (Utilities|Casting|CastToBP_HUD_ATBTT (HUD|GetHUD (Game|GetPlayerController 0)))
        (:then
          (Default|DisplayCenterText (Variables|/Game/AdvancedTurnBasedTileToolkit/Core/UI/BP_HUD_ATBTT.BP_HUD_ATBTT_C|GetWbpAtbttRef _asbp_hud_atbtt) (Variables|Default|GetDisplayText) 0.0)
          (CallFunction|EndAction true))
        (:CastFailed
          (goto _label))))))

(fn ConstructionScript
  (|CallParentFunction))